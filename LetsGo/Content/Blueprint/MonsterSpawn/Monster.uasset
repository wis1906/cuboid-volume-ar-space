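; Monster actor that walks a route of points and destroys itself after reaching the last one.
; CheckStart turns it toward the first point and enables movement, which Tick applies as a fixed, unswept step not scaled by delta time.
; Within a small distance of each point, it advances the index and yaws BoxCollision toward the next using a look-at rotation with a -90 degree offset.
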(event `self.ReceiveBeginPlay`)

(event `CheckStart`
  (`self.RotateToDest` (`|GetArrayItem` (`self.routePoints`)))
  (set `self.isMoveStart` true))

(event `self.ReceiveTick`
  (params (DeltaSeconds :type "Float (single-precision)"))
  (if (`self.isMoveStart`)
    (if (< (`self.curRouteIdx`) (`KismetArrayLibrary.Array_Length` (`self.routePoints`)))
      (`self.MoveToDest` (`|GetArrayItem` (`self.routePoints`) (`self.curRouteIdx`))))))

(event `MoveToDest`
  (params (dest :type "Vector Structure"))
  (`self.K2_AddActorWorldTransform` (`KismetMathLibrary.MakeTransform` (* (`KismetMathLibrary.Normal` (- dest (`self.K2_GetActorLocation`))) (`self.movingSpeed`))))
  (`self.CheckDist` dest))

(event `RotateToDest`
  (params (Dest :type "Vector Structure"))
  (bind _boxcollision (`self.BoxCollision`))
  (`SceneComponent.K2_AddLocalRotation` _boxcollision (`KismetMathLibrary.MakeRotator` 0.0 0.0 (+ (.yaw (`KismetMathLibrary.InverseTransformRotation` (`SceneComponent.K2_GetComponentToWorld` _boxcollision) (`KismetMathLibrary.FindLookAtRotation` (`SceneComponent.K2_GetComponentLocation` _boxcollision) Dest))) -90.0)) false false))

(event `CheckDist`
  (params (dest :type "Vector Structure"))
  (if (<= (`KismetMathLibrary.VSize` (- dest (`self.K2_GetActorLocation`))) 20.0)
    (`/Engine/EditorBlueprintResources/StandardMacros.IncrementInt` (`self.curRouteIdx`)
      (:`  `
        (if (< (`self.curRouteIdx`) (`KismetArrayLibrary.Array_Length` (`self.routePoints`)))
          (`self.RotateToDest` (`|GetArrayItem` (`self.routePoints`) (`self.curRouteIdx`)))
          (else
            (`self.K2_DestroyActor`)))))))

(fn `UserConstructionScript`)