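; BP_MonsterSpawnMgr is a manager Blueprint that launches monster spawning along routes.
; SpawnMonsterbyRoute creates a BP_MonsterSpawner at the world origin, passes it the rotation, entry, route and exit points and monster type, then calls StartSpawn, leaving the spawning itself to that actor.
; A separate DrawBoxLine event draws long-lived colored debug lines between two positions.
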(event `self.drawBoxLine`
  (params (startPos :type "Vector Structure") (destPos :type "Vector Structure") (c :type "Color Structure"))
  (`KismetSystemLibrary.DrawDebugLine` startPos destPos (`KismetMathLibrary.Conv_ColorToLinearColor` c) 100000.0 5.0))

(event `self.spawnMonsterByRoute`
  (params (rotation :type "Rotator Structure") (entryPoint :type "Vector Structure") (routePoint :type "Array of Vector Structure (by ref)") (exitPoint :type "Vector Structure") (monsterType :type Integer))
  (bind _returnvalue (`|SpawnActorFromClass` "/Game/Blueprint/MonsterSpawn/BP_MonsterSpawner.BP_MonsterSpawner_C" (`KismetMathLibrary.MakeTransform` (0.0 0.0 0.0)) "Undefined" "OverrideRootScale" null null))
  (set `/Game/Blueprint/MonsterSpawn/BP_MonsterSpawner.Rotation` rotation _returnvalue)
  (set `/Game/Blueprint/MonsterSpawn/BP_MonsterSpawner.EntryPoint` entryPoint _returnvalue)
  (set `/Game/Blueprint/MonsterSpawn/BP_MonsterSpawner.RoutePoint` routePoint _returnvalue)
  (set `/Game/Blueprint/MonsterSpawn/BP_MonsterSpawner.ExitPoint` exitPoint _returnvalue)
  (set `/Game/Blueprint/MonsterSpawn/BP_MonsterSpawner.monsterType` monsterType _returnvalue)
  (`/Game/Blueprint/MonsterSpawn/BP_MonsterSpawner.StartSpawn` _returnvalue))

(fn `UserConstructionScript`)