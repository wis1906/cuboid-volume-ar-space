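; SLAM manager Blueprint that visualizes landmarks, keyframes and the camera path in the world with long-lived debug drawing.
; Draw events plot landmarks as small points colored by outlier status, keyframes as larger red points, and frame cameras as line segments chained through PrevCamPos.
; All three events draw nothing while IsSpawnMonster is set.
; Alternative debug shapes and red/green point-actor spawns remain as unconnected nodes.
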(event `self.drawLandmark`
  (params (pos :type "Vector Structure") (isOutlier :type Boolean))
  (if (`self.isSpawnMonster`)
    _
    (elif isOutlier
      (`KismetSystemLibrary.DrawDebugPoint` pos 3.0 (struct :`A` 1.0) 10000.0)
      (else
        (`KismetSystemLibrary.DrawDebugPoint` pos 3.0 (struct :`G` 1.0 :`A` 1.0) 10000.0)))))

(event `self.drawKeyframeCamera`
  (params (pos :type "Vector Structure"))
  (if (not (`self.isSpawnMonster`))
    (`KismetSystemLibrary.DrawDebugPoint` pos 10.0 (struct :`R` 1.0 :`A` 1.0) 10000.0)))

(event `self.drawFrameCamera`
  (params (pos :type "Vector Structure"))
  (if (not (`self.isSpawnMonster`))
    (`KismetSystemLibrary.DrawDebugLine` (`self.prevCamPos`) pos (struct :`R` 1.0 :`G` 0.920947 :`A` 1.0) 10000.0 2.0)
    (set `self.prevCamPos` pos)))

(fn `UserConstructionScript`)