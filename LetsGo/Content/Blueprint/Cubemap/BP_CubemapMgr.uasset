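; BP_CubemapMgr manages a six-sided cubemap display whose face textures refresh with video frames.
; On BeginPlay it creates a dynamic material instance for each of the Top, Bottom, Rear, Left, Front and Right components from per-face source materials.
; Each OnNextVideoFrame event pushes the matching face texture variable into that instance's "Texture" parameter.
; The file does not assign those texture variables itself.
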(event `self.ReceiveBeginPlay`
  (bind _returnvalue (`PrimitiveComponent.CreateDynamicMaterialInstance` (`self.Top`) 0 "/Game/Material/Cubemap/M_Top.M_Top"))
  (set `self.DMTop` _returnvalue)
  (bind _returnvalue_2 (`PrimitiveComponent.CreateDynamicMaterialInstance` (`self.Bottom`) 0 "/Game/Material/Cubemap/M_Bottom.M_Bottom"))
  (set `self.DMBottom` _returnvalue_2)
  (bind _returnvalue_3 (`PrimitiveComponent.CreateDynamicMaterialInstance` (`self.Rear`) 0 "/Game/Material/Cubemap/M_Rear.M_Rear"))
  (set `self.DMRear` _returnvalue_3)
  (bind _returnvalue_4 (`PrimitiveComponent.CreateDynamicMaterialInstance` (`self.Left`) 0 "/Game/Material/Cubemap/M_Left.M_Left"))
  (set `self.DMLeft` _returnvalue_4)
  (bind _returnvalue_5 (`PrimitiveComponent.CreateDynamicMaterialInstance` (`self.Front`) 0 "/Game/Material/Cubemap/M_Front.M_Front"))
  (set `self.DMFront` _returnvalue_5)
  (bind _returnvalue_6 (`PrimitiveComponent.CreateDynamicMaterialInstance` (`self.Right`) 0 "/Game/Material/Cubemap/M_Right.M_Right"))
  (set `self.DMRight` _returnvalue_6))

(event `self.OnNextVideoFrame`
  (`MaterialInstanceDynamic.SetTextureParameterValue` (`self.DMTop`) "Texture" (`self.TopTexture`))
  (`MaterialInstanceDynamic.SetTextureParameterValue` (`self.DMBottom`) "Texture" (`self.BottomTexture`))
  (`MaterialInstanceDynamic.SetTextureParameterValue` (`self.DMRear`) "Texture" (`self.RearTexture`))
  (`MaterialInstanceDynamic.SetTextureParameterValue` (`self.DMLeft`) "Texture" (`self.LeftTexture`))
  (`MaterialInstanceDynamic.SetTextureParameterValue` (`self.DMFront`) "Texture" (`self.FrontTexture`))
  (`MaterialInstanceDynamic.SetTextureParameterValue` (`self.DMRight`) "Texture" (`self.RightTexture`)))

(fn `UserConstructionScript`)